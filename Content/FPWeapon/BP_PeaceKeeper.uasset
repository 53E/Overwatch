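; BP_PeaceKeeper is a first-person weapon Blueprint that animates its own recoil by rotating the scene root.
; Recoil kicks the roll up, by a fixed amount for fan fire or by RecoolRange for a normal shot.
; Looping timers then step it back down through DoN counters.
; The fan-fire timer is faster and clears at its step limit, while the normal timer clears after a delay.
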(event Custom|AddFan
  (bind _counter (Utilities|FlowControl|DoN 50)
    (:Exit
      (if (== _counter 50)
        (Utilities|Time|ClearandInvalidateTimerbyHandle (stale EventRecoil _returnvalue))
        (else
          (Transformation|AddRelativeRotation (Variables|Default|GetDefaultSceneRoot) (Math|Rotator|MakeRotator -0.1 0.0 0.0) false false))))))

(event Custom|Add
  (Utilities|FlowControl|DoN 50
    (:Exit
      (Transformation|AddRelativeRotation (Variables|Default|GetDefaultSceneRoot) (Math|Rotator|MakeRotator -0.2 0.0 0.0) false false))))

(event EventRecoil
  (params (bIsFanFire :type Boolean))
  (if bIsFanFire
    (Utilities|FlowControl|Sequence
      (:then_0
        (Utilities|FlowControl|DoN 50) ; enters at Reset
      )
      (:then_1
        (Transformation|AddRelativeRotation (Variables|Default|GetDefaultSceneRoot) (Math|Rotator|MakeRotator 5.0 0.0 0.0) false false)
        (bind _returnvalue (Utilities|Time|SetTimerbyEvent (delegate Custom|AddFan) 0.0025 true))))
    (else
      (Utilities|FlowControl|Sequence
        (:then_0
          (Utilities|FlowControl|DoN 50) ; enters at Reset
        )
        (:then_1
          (Transformation|AddRelativeRotation (Variables|Default|GetDefaultSceneRoot) (Math|Rotator|MakeRotator (Variables|Default|GetRecoolRange) 0.0 0.0) false false)
          (bind _returnvalue_2 (Utilities|Time|SetTimerbyEvent (delegate Custom|Add) 0.008 true))
          (Utilities|FlowControl|Delay 0.45)
          (Utilities|Time|ClearandInvalidateTimerbyHandle _returnvalue_2))))))

(fn ConstructionScript)