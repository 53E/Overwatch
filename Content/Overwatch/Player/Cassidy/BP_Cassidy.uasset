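; Player Blueprint for Cassidy, handling the presentation side of the hero's pistol shots, Fan Fire, dodge roll and High Noon.
; Creates the HUD widget for the local player, then drives its hit and Fan Fire feedback through events and a timer.
; Timelines apply recoil pitch and dodge camera dip, alongside randomized fire sounds and the roll montage.
; High Noon maps each target to a screen-projected progress widget, updated and cleared by events.
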(event Custom|MulticastPlayRoll
  (Animation|Montage|PlayMontage (Variables|Character|GetMesh) "/Game/Overwatch/Animation/Mixamo/Anim/Pistol_roll1_Montage.Pistol_roll1_Montage" 2.1))

(event EventBeginPlay
  (|BeginPlay))

(event EventFireSoundEcho
  (|EchoSound))

(event EventHitUI
  (params (IsHead :type Boolean))
  (bind _returnvalue (Transformation|GetActorLocation))
  (bind _cassidywidget (Variables|Default|GetCassidyWidget))
  (if IsHead
    (Default|EventHitBig _cassidywidget)
    (Audio|PlaySoundatLocation "/Game/Overwatch/Sound/Cassidy/Hit/HeadShotSound.HeadShotSound" (Transformation|GetActorLocation) "0, 0, 0" 1.0 1.0 0.0 0 0 0 0)
    (else
      (Default|EventHitSmall _cassidywidget)
      (Utilities|FlowControl|FlipFlop
        (:A
          (Audio|PlaySoundatLocation "/Game/Overwatch/Sound/Cassidy/Hit/HitSound01.HitSound01" _returnvalue "0, 0, 0" 1.0 1.0 0.0 0 0 0 0))
        (:B
          (Audio|PlaySoundatLocation "/Game/Overwatch/Sound/Cassidy/Hit/HitSound02.HitSound02" _returnvalue "0, 0, 0" 1.0 1.0 0.0 0 0 0 0))))))

(event EventDodgeMontage
  (CallFunction|MulticastPlayRoll))

(event EventDownCameraonDodge
  (|DownCamera))

(event EventRecoil
  (params (bIsFanFire :type Boolean))
  (|RecoilNode bIsFanFire))

(event EventFanFireUI
  (params (time :type Float%20%28single-precision%29))
  (|FanFireUINODE time))

(event EventShowHighnoonTargetUI
  (params (Target :type Actor%20Object%20Reference) (InitialSize :type Float%20%28single-precision%29))
  (bind _returnvalue (UserInterface|CreateWidget "/Game/Overwatch/UI/InGame/WB_Highnoon.WB_Highnoon_C"))
  (Utilities|Map|Add (Variables|Default|GetMap) Target _returnvalue)
  (Class|UserWidget|SetPositioninViewport _returnvalue (.ScreenPosition (Class|GameplayStatics|ProjectWorldtoScreen (Game|GetPlayerController 0) (Transformation|GetActorLocation Target) false)) true)
  (UserInterface|Viewport|AddtoViewport _returnvalue 0))

(event EventHideHighnoonTargetUI
  (params (Target :type Actor%20Object%20Reference))
  (bind _map (Variables|Default|GetMap))
  (bind _values (Utilities|Map|Values _map))
  (for _array_element _values
    (Widget|RemovefromParent _array_element))
  (Utilities|Map|Clear _map))

(event EventOnHighnoonReady)

(event EventUpdateHighnoonTargetUI
  (params (Target :type Actor%20Object%20Reference) (Progress :type Float%20%28single-precision%29))
  (bind _map (Variables|Default|GetMap))
  (bind (_value _returnvalue) (Utilities|Map|Find _map Target))
  (if _returnvalue
    (Default|ProgressCircle _value)
    (Class|UserWidget|SetPositioninViewport _value (.ScreenPosition (Class|GameplayStatics|ProjectWorldtoScreen (Game|GetPlayerController 0) (Transformation|GetActorLocation Target) false)) true)))

(fn ConstructionScript)

(event Custom|DoFanFireAnim
  (if (Utilities|Time|IsValidTimerHandle (stale _returnvalue))
    (Default|FanFireAnim (Variables|Default|GetCassidyWidget))
    (Utilities|Time|ClearandInvalidateTimerbyHandle (stale _returnvalue))))

(event EventStopFanFireUI
  (Default|DodgeAnim (Variables|Default|GetCassidyWidget)))